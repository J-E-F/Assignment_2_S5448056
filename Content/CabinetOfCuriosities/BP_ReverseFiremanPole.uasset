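; An interactable reverse fireman pole that carries the first-person player between a bottom and a top point.
; Interact checks which end collider the player overlaps, then calls MoveToTop or MoveToBottom, which set a moving flag and disable input on the pole.
; Timelines lerp the player's location to the opposite point after a lever sound plays.
; A text prompt shows only while the bottom collider is overlapped.
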(event OnComponentBeginOverlap(Bottom_Collider)
  (params (OverlappedComponent :type Primitive%20Component%20Object%20Reference) (OtherActor :type Actor%20Object%20Reference) (OtherComp :type Primitive%20Component%20Object%20Reference) (OtherBodyIndex :type Integer) (bFromSweep :type Boolean) (SweepResult :type Hit%20Result%20Structure%20%28by%20ref%29))
  (Rendering|SetVisibility (Variables|Default|GetTextRender) true false))

(event OnComponentEndOverlap(Bottom_Collider)
  (params (OverlappedComponent :type Primitive%20Component%20Object%20Reference) (OtherActor :type Actor%20Object%20Reference) (OtherComp :type Primitive%20Component%20Object%20Reference) (OtherBodyIndex :type Integer))
  (Rendering|SetVisibility (Variables|Default|GetTextRender) false false))

(event Custom|MovePlayerToTop
  (Audio|PlaySound2D "/Game/Sounds/Mechanical__Lever__Wooden_Lever__Slide_Into_Place_02_SND144269.Mechanical__Lever__Wooden_Lever__Slide_Into_Place_02_SND144269" 1.0 1.0 0.0 0 0)
  (bind _alpha (Timeline|TL_MoveToTop PlayFromStart)
    (:Update
      (Transformation|SetActorLocation (Game|GetPlayerCharacter 0) (Math|Vector|Lerp(Vector) (Variables|Default|GetPlayerLocation) (Transformation|GetWorldLocation (Variables|Default|GetTop%20Point)) _alpha) false false)
      (Variables|Default|SetIsMoving false)
      (Components|Activation|Activate (Variables|/Script/Engine.Actor|GetRootComponent (Game|GetPlayerController 0)) false))))

(event Custom|MovePlayerToBottom
  (Audio|PlaySound2D "/Game/Sounds/Mechanical__Lever__Wooden_Lever__Slide_Into_Place_02_SND144269.Mechanical__Lever__Wooden_Lever__Slide_Into_Place_02_SND144269" 1.0 1.0 0.0 0 0)
  (bind _alpha (Timeline|TL_MoveToBottom PlayFromStart)
    (:Update
      (Transformation|SetActorLocation (Game|GetPlayerCharacter 0) (Math|Vector|Lerp(Vector) (Variables|Default|GetPlayerLocation) (Transformation|GetWorldLocation (Variables|Default|GetBottom%20Point)) _alpha) false false)
      (Variables|Default|SetIsMoving false)
      (Components|Activation|Activate (Variables|/Script/Engine.Actor|GetRootComponent (Game|GetPlayerController 0)) false))))

(event EventInteract
  (params (Insitgator :type BP%20First%20Person%20Character%20Object%20Reference))
  (bind _returnvalue (Game|GetPlayerCharacter 0))
  (if (not (Variables|Default|GetIsMoving))
    (Variables|Default|SetPlayerLocation (Transformation|GetActorLocation (Game|GetPlayerCharacter 0)))
    (if (Utilities|Array|ContainsItem (Collision|GetOverlappingActors (Variables|Default|GetBottom_Collider) "/Game/FirstPerson/Blueprints/BP_FirstPersonCharacter.BP_FirstPersonCharacter_C" :!class /Script/Engine.PrimitiveComponent) _returnvalue)
      (CallFunction|MovetoTop)
      (elif (Utilities|Array|ContainsItem (Collision|GetOverlappingActors (Variables|Default|GetTop_Collider) "/Game/FirstPerson/Blueprints/BP_FirstPersonCharacter.BP_FirstPersonCharacter_C" :!class /Script/Engine.PrimitiveComponent) _returnvalue)
        (CallFunction|MovetoBottom)))))

(event EventBeginPlay
  (Rendering|SetVisibility (Variables|Default|GetTextRender) false false))

(fn ConstructionScript)

(fn MovetoTop
  (Variables|Default|SetIsMoving true)
  (Input|DisableInput (Game|GetPlayerController 0))
  (CallFunction|MovePlayertoTop))

(fn MovetoBottom
  (Variables|Default|SetIsMoving true)
  (Input|DisableInput (Game|GetPlayerController 0))
  (CallFunction|MovePlayertoBottom))

(fn OnInteract)