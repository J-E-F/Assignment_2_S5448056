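; A ball actor that a player can pick up, with a text prompt shown on proximity.
; Overlapping SphereCollider1 while the ball is not held shows the text, detaches that collider and makes it visible in game; leaving hides the text.
; Interact stores the instigator as Holder, marks the ball held, disables its physics and collision, then hands it to the instigator through PlayerInteract.
; The ball starts with physics off, and no release logic exists here.
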(event OnComponentBeginOverlap(SphereCollider1)
  (params (OverlappedComponent :type Primitive%20Component%20Object%20Reference) (OtherActor :type Actor%20Object%20Reference) (OtherComp :type Primitive%20Component%20Object%20Reference) (OtherBodyIndex :type Integer) (bFromSweep :type Boolean) (SweepResult :type Hit%20Result%20Structure%20%28by%20ref%29))
  (bind _spherecollider1 (Variables|Default|GetSphereCollider1))
  (if (not (Variables|Default|GetIsHeld))
    (Rendering|SetVisibility (Variables|Default|GetTextRender) true false)
    (Transformation|DetachFromComponent _spherecollider1 "KeepRelative" "KeepRelative" "KeepRelative" true)
    (Development|SetHiddeninGame _spherecollider1 false false)))

(event OnComponentEndOverlap(SphereCollider1)
  (params (OverlappedComponent :type Primitive%20Component%20Object%20Reference) (OtherActor :type Actor%20Object%20Reference) (OtherComp :type Primitive%20Component%20Object%20Reference) (OtherBodyIndex :type Integer))
  (Rendering|SetVisibility (Variables|Default|GetTextRender) false false))

(event EventBeginPlay
  (Physics|SetSimulatePhysics (Variables|Default|GetBall) false)
  (Rendering|SetVisibility (Variables|Default|GetTextRender) false false)
  (Variables|Default|SetIsHeld false))

(event EventTick
  (params (DeltaSeconds :type Float%20%28single-precision%29)))

(event EventInteract
  (params (Insitgator :type BP%20First%20Person%20Character%20Object%20Reference))
  (bind _ball (Variables|Default|GetBall))
  (Variables|Default|SetHolder Insitgator)
  (Variables|Default|SetIsHeld true)
  (Physics|SetSimulatePhysics _ball false)
  (Collision|SetCollisionEnabled _ball "NoCollision")
  (Default|PlayerInteract Insitgator self))

(fn ConstructionScript)